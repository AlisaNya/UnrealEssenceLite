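; BP_Demo is a demo actor that exercises the WBP_TypeWriter typing-effect widget.
; On BeginPlay it enables input, adds the widget to the viewport with left-to-right direction and auto-justify off, and binds its end-of-typing event to a debug print.
; E starts the typing effect and Q changes its direction for testing.
; Unconnected nodes hold other widget settings and a stop call that are never executed.
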(event Collision|EventActorBeginOverlap
  (params (OtherActor :type Actor%20Object%20Reference)))

(event EventTick
  (params (DeltaSeconds :type Float%20%28single-precision%29)))

(event Custom|OnAllAllowedCharsIsEndTyping_Event
  (Development|PrintString "Hello"))

(event EventBeginPlay
  (bind _returnvalue (Game|GetPlayerController 0))
  (Input|EnableInput _returnvalue)
  (bind _returnvalue_2 (UserInterface|CreateWidget "/UnrealEssenceLite/WBP_TypeWriter.WBP_TypeWriter_C" _returnvalue))
  (bind _output_get (Variables|Default|SetWBP _returnvalue_2))
  (UserInterface|Viewport|AddtoViewport _output_get 0)
  (Class|TypingEffectWidget|SetDirection (Variables|Default|GetWBP) "LeftToRight")
  (Variables|/Script/UnrealEssenceLite.TypingEffectWidget|SetbJustifyIsAuto (Variables|Default|GetWBP) false)
  (EventDispatchers|AssignOnAllAllowedCharsIsEndTyping (Variables|Default|GetWBP) (delegate Custom|OnAllAllowedCharsIsEndTyping_Event)))

(event Input|KeyboardEvents|E
  (params (Key :type Key%20Structure :default "None"))
  (:Pressed
    (Class|TypingEffectWidget|StartTypingEffect (Variables|Default|GetWBP) false false)))

(event Input|KeyboardEvents|Q
  (params (Key :type Key%20Structure :default "None"))
  (:Pressed
    (Class|TypingEffectWidget|ChangeDirection (Variables|Default|GetWBP)) ; меняем направление после каждой остановки для теста
  ))

(fn ConstructionScript)